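; Level-kit optimizer volume that replaces static mesh actors inside its box with instanced static mesh components.
; TraceBox runs a Visibility box trace and keeps meshes matching the StaticMesh list, or all when IgnoreArray is set, though only filtered hits return as actors.
; BeginPlay converts unless IsInit is set, then destroys those returned actors.
; Reset destroys the generated instance components; Hide is an empty stub.
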(event Custom|ConstructionUpdated
  (Components|Box|SetBoxExtent (Variables|Default|GetBox) (Variables|AConfig|GetIn%20Box%20Extent) true))

(event EventBeginPlay
  (if (Variables|Base|GetIsInit)
    _
    (else
      (Base|Convert false)))
  (bind (_success _outhits _staticmesheactors) (Base|TraceBox))
  (if _success
    (for _array_element _staticmesheactors
      (Utilities|IsValid _array_element
        (:Is%20Valid
          (Actor|DestroyActor _array_element))))
    (Utilities|Array|Clear (Variables|AConfig|GetStatic%20Mesh))))

(fn ConstructionScript
  (CallFunction|ConstructionUpdated))

(fn Convert
  (params (Hide :type Boolean))
  (bind (_success _outhits _staticmesheactors _staticmeshcomponents) (Base|TraceBox))
  (if _success
    (bind (_success_2 _instancestaticmeshes) (CallFunction|ConvertSMCtoISMC self _staticmeshcomponents false false "Static"))
    (if _success_2
      (Variables|Base|SetInstance%20Static%20Meshes _instancestaticmeshes)
      (if Hide
        (Base|Hide true)))))

(fn TraceBox
  (bind _staticmeshactor (LocalVariables|GetStaticMeshActor))
  (bind _staticmeshcomponent (LocalVariables|GetStaticMeshComponent))
  (bind _scene (Variables|Default|GetScene))
  (bind _returnvalue (Transformation|GetWorldLocation _scene))
  (for _array_element (Variables|AConfig|GetStatic%20Mesh)
    (Utilities|Array|Add (LocalVariables|GetCheckStaticMeshes) (Variables|/Script/Engine.StaticMeshComponent|GetStaticMesh (Variables|/Script/Engine.StaticMeshActor|GetStaticMeshComponent _array_element))))
  (bind (_outhits _returnvalue_2) (Class|KismetSystemLibrary|BoxTraceMulti _returnvalue _returnvalue (Variables|AConfig|GetIn%20Box%20Extent) "0, 0, 0" "TraceTypeQuery1" false 0 "ForOneFrame" true))
  (for _array_element_2 _outhits
    (bind _asstatic_mesh_actor (Utilities|Casting|CastToStaticMeshActor (.HitActor (Collision|BreakHitResult _array_element_2))))
    (if (Variables|AConfig|GetIgnoreArray?)
      (Utilities|Array|Add _staticmeshcomponent (Variables|/Script/Engine.StaticMeshActor|GetStaticMeshComponent _asstatic_mesh_actor) :!label _label)
      (elif (not (== (Utilities|Array|FindItem (LocalVariables|GetCheckStaticMeshes) (Variables|/Script/Engine.StaticMeshComponent|GetStaticMesh (Variables|/Script/Engine.StaticMeshActor|GetStaticMeshComponent _asstatic_mesh_actor))) -1))
        (Utilities|Array|Add _staticmeshactor _asstatic_mesh_actor)
        (goto _label))))
  (return _returnvalue_2 _outhits _staticmeshactor _staticmeshcomponent))

(fn Hide
  (params (bNewHidden :type Boolean)))

(fn Reset
  (bind _instance_static_meshes (Variables|Base|GetInstance%20Static%20Meshes))
  (Base|Hide false)
  (for _array_element _instance_static_meshes
    (Components|DestroyComponent _array_element)
    (Utilities|Array|Clear _instance_static_meshes)))