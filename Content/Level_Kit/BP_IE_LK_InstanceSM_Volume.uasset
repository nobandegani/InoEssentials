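; Box volume that replaces StaticMeshActors inside it with instanced static mesh components, run on BeginPlay when enabled.
; A box trace gathers actors, optionally filtered to selected actors' meshes, recording mesh and transform.
; Meshes meeting a minimum count get a static ISM component with cull distances; material overrides are not copied.
; Converted actors are tagged with the volume's name, then destroyed by tag lookup.
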(event Custom|OnConstruction
  ;[1 1 1] OnConstruction
  (Components|Box|SetBoxExtent (Variables|Default|GetBox) (Variables|AConfig|GetIn%20Box%20Extent) true))

(event Custom|CreateInstances
  (bind _box (Variables|Default|GetBox))
  (bind _traceactorsref (Variables|Trace|GetTraceActorsRef))
  (bind _uniquestaticmeshes (Variables|InstanceReq|GetUniqueStaticMeshes))
  (bind _returnvalue (Transformation|GetWorldLocation _box))
  ;[1 1 1] Create instances
  (CallFunction|Reset)
  (if (Variables|AConfig|GetCustomMeshes)
    (for _array_element (Variables|AConfig|GetSelectedActors)
      (Utilities|Array|AddUnique (Variables|Base|GetSelectedStaticMeshes) (Variables|/Script/Engine.StaticMeshComponent|GetStaticMesh (Variables|/Script/Engine.StaticMeshActor|GetStaticMeshComponent _array_element)))))
  (bind (_outhits _returnvalue_2) (Base|MultiBoxTrace _returnvalue _returnvalue (Variables|/Script/Engine.BoxComponent|GetBoxExtent _box)))
  (if _returnvalue_2
    (for _array_element_2 _outhits
      (if (and (== (Utilities|GetClass (.HitActor (Collision|BreakHitResult _array_element_2))) "/Script/Engine.StaticMeshActor") (== (Utilities|GetClass (.HitComponent (Collision|BreakHitResult _array_element_2))) "/Script/Engine.StaticMeshComponent"))
        (bind _returnvalue_3 (Utilities|Array|AddUnique (Variables|Trace|GetTraceActorsNames) (Utilities|GetObjectName (.HitActor (Collision|BreakHitResult _array_element_2)))))
        (if (not (== _returnvalue_3 -1))
          (bind _asstatic_mesh_component (Utilities|Casting|CastToStaticMeshComponent (.HitComponent (Collision|BreakHitResult _array_element_2))))
          (Utilities|IsValid (Variables|/Script/Engine.StaticMeshComponent|GetStaticMesh _asstatic_mesh_component)
            (:Is%20Valid
              (if (Variables|AConfig|GetCustomMeshes)
                (if (not (== (Utilities|Array|FindItem (Variables|Base|GetSelectedStaticMeshes) (Variables|/Script/Engine.StaticMeshComponent|GetStaticMesh _asstatic_mesh_component)) -1))
                  (bind _returnvalue_4 (Utilities|Array|AddUnique _traceactorsref (.HitActor (Collision|BreakHitResult _array_element_2)) :!label _label))
                  (bind _returnvalue_5 (Utilities|Array|AddUnique _uniquestaticmeshes (Variables|/Script/Engine.StaticMeshComponent|GetStaticMesh _asstatic_mesh_component)))
                  (Utilities|Array|Add (Variables|InstanceReq|GetInstances) (Utilities|Struct|MakeST_LK_ISM_Metadata (select (== _returnvalue_5 -1) (Utilities|Array|FindItem _uniquestaticmeshes (Variables|/Script/Engine.StaticMeshComponent|GetStaticMesh _asstatic_mesh_component)) _returnvalue_5) 0 (select (== _returnvalue_4 -1) _returnvalue_4 (Utilities|Array|FindItem _traceactorsref (.HitActor (Collision|BreakHitResult _array_element_2)))) (Transformation|GetActorTransform (.HitActor (Collision|BreakHitResult _array_element_2)))))
                  (Class|FLBase|InoLog (Utilities|String|Append "instance " (Utilities|GetObjectName (.HitActor (Collision|BreakHitResult _array_element_2))) " added") 5.0 "(TagName=\"Ino.Log.Type.Info\")" "(TagName=\"Ino.Log.Category.Unkown\")"))
                (else
                  (goto _label))))
            (:Is%20Not%20Valid
              (Class|FLBase|InoLog "invalid mesh" 5.0 "(TagName=\"Ino.Log.Type.Error\")" "(TagName=\"Ino.Log.Category.Unkown\")"))))))
    (Class|FLBase|InoLog (Utilities|String|Append "no unique meshes: " (Utilities|String|ToString(Integer) (Utilities|Array|Length (Variables|InstanceReq|GetUniqueStaticMeshes))) "--" "no instances: " (Utilities|String|ToString(Integer) (Utilities|Array|Length (Variables|InstanceReq|GetInstances)))) 15.0 "(TagName=\"\")" "(TagName=\"Ino\")")
    (for (_array_element_3 _array_index) (Variables|InstanceReq|GetUniqueStaticMeshes)
      (if (Base|IsMoreThanMax _array_index)
        (bind _returnvalue_6 (AddComponent|AddInstancedStaticMeshComponent false))
        (Transformation|SetMobility _returnvalue_6 "Static")
        (Components|InstancedStaticMesh|SetCullDistances _returnvalue_6 (Variables|AConfig|GetStart%20Cull%20Distance) (Variables|AConfig|GetEnd%20Cull%20Distance))
        (Utilities|Map|Add (Variables|Instance|GetInstancesRef) _array_index _returnvalue_6)
        (Components|StaticMesh|SetStaticMesh _returnvalue_6 _array_element_3)))
    (bind _array_element_4 (Utilities|Array|ForEachLoopwithBreak (Variables|InstanceReq|GetInstances))
      (:LoopBody
        (if (.ReturnValue (Utilities|Map|Find (Variables|Instance|GetInstancesRef) (.StaticMeshIndex (Utilities|Struct|BreakST_LK_ISM_Metadata _array_element_4))))
          (Components|InstancedStaticMesh|AddInstance (.Value (Utilities|Map|Find (Variables|Instance|GetInstancesRef) (.StaticMeshIndex (Utilities|Struct|BreakST_LK_ISM_Metadata _array_element_4)))) (.Transform (Utilities|Struct|BreakST_LK_ISM_Metadata _array_element_4)) true)
          (Utilities|Array|AddUnique (Variables|/Script/Engine.Actor|GetTags (Utilities|Array|Get(acopy) (Variables|Trace|GetTraceActorsRef) (.ActorIndex (Utilities|Struct|BreakST_LK_ISM_Metadata _array_element_4)))) (Base|GetObjectName))
          (Variables|/Script/Engine.Actor|SetTags (Utilities|Array|Get(acopy) (Variables|Trace|GetTraceActorsRef) (.ActorIndex (Utilities|Struct|BreakST_LK_ISM_Metadata _array_element_4))) (Variables|/Script/Engine.Actor|GetTags (Utilities|Array|Get(acopy) (Variables|Trace|GetTraceActorsRef) (.ActorIndex (Utilities|Struct|BreakST_LK_ISM_Metadata _array_element_4)))))))
      (:Completed
        (CallFunction|Delete)
        (CallFunction|ClearBase)
        (CallFunction|ClearInstanceReq)
        (CallFunction|ClearTraceRef)
        (CallFunction|ClearConfig)))
    (else
      (Class|FLBase|InoLog "no hit" 5.0 "(TagName=\"Ino.Log.Type.Error\")" "(TagName=\"Ino.Log.Category.Unkown\")"))))

(event Custom|Reset
  ;[1 1 1] Reset
  (CallFunction|ClearInstances)
  (CallFunction|ClearBase)
  (CallFunction|ClearInstanceReq)
  (CallFunction|ClearTraceRef))

(event Custom|Delete
  ;[1 1 1] Delete
  (bind _outactors (Actor|GetAllActorsOfClass "/Script/Engine.StaticMeshActor"))
  (for _array_element _outactors
    (if (not (== (Utilities|Array|FindItem (Variables|/Script/Engine.Actor|GetTags _array_element) (Base|GetObjectName)) -1))
      (Actor|DestroyActor _array_element))))

(event Custom|ClearTraceRef
  ;[1 1 1] Clear
  (Utilities|Array|Clear (Variables|Trace|GetTraceActorsNames))
  (Utilities|Array|Clear (Variables|Trace|GetTraceActorsRef)))

(event Custom|ClearInstanceReq
  ;[1 1 1] Clear
  (Utilities|Array|Clear (Variables|InstanceReq|GetUniqueStaticMeshes))
  (Utilities|Array|Clear (Variables|InstanceReq|GetUniqueMaterialSet))
  (Utilities|Array|Clear (Variables|InstanceReq|GetInstances)))

(event Custom|ClearBase
  ;[1 1 1] Clear
  (Utilities|Array|Clear (Variables|Base|GetSelectedStaticMeshes)))

(event Custom|ClearInstances
  (bind _instancesref (Variables|Instance|GetInstancesRef))
  ;[1 1 1] Clear
  (bind _values (Utilities|Map|Values _instancesref))
  (Components|InstancedStaticMesh|ClearInstances _values)
  (Components|DestroyComponent _values)
  (Utilities|Map|Clear _instancesref))

(event Custom|ClearConfig
  ;[1 1 1] Clear
  (Utilities|Array|Clear (Variables|AConfig|GetSelectedActors)))

(event EventBeginPlay
  (if (Variables|AConfig|GetEnable?)
    (CallFunction|CreateInstances)))

(fn ConstructionScript
  (CallFunction|OnConstruction))

(fn GetNumberOfInstances
  (params (Index :type Integer))
  (bind _newlocalvar (LocalVariables|GetNewLocalVar))
  (for _array_element (Variables|InstanceReq|GetInstances)
    (if (== Index (.StaticMeshIndex (Utilities|Struct|BreakST_LK_ISM_Metadata _array_element)))
      (Math|Integer|IncrementInt _newlocalvar)))
  (return _newlocalvar))

(fn MultiBoxTrace
  (params (Start :type Vector) (End :type Vector) (HalfSize :type Vector))
  (bind (_outhits _returnvalue) (Class|KismetSystemLibrary|BoxTraceMultiforObjects Start End HalfSize "0, 0, 0" (Variables|AConfig|GetObject%20Types) false 0 "None" true))
  (return _outhits _returnvalue))

(fn IsMoreThanMax
  (params (Index :type Integer))
  (return (>= (Base|GetNumberOfInstances Index) (Variables|AConfig|GetMiniumToInstance))))

(fn GetObjectName
  (return (Utilities|String|StringToName (Utilities|GetObjectName self))))