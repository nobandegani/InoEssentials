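; Level Kit actor component that optimizes its owner by converting StaticMeshComponents into InstancedStaticMeshComponents, at BeginPlay if AutoOptimize is set or through Setup.
; Convert creates one instanced component per unique mesh, using the first source's materials, then adds each source's world transform as an instance.
; It optionally deletes or hides sources and runs once unless IgnoreInit is set.
; Both ConvertSMToInstanceSM functions are empty, with older logic left disconnected.
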(event EventBeginPlay
  (if (Variables|Default|GetAutoOptimize)
    (Base|Convert (Actor|GetComponentsByClass (Components|GetOwner) "/Script/Engine.StaticMeshComponent") true false false "Static")))

(fn ConvertStaticMaterialArraytoMaterialInterfaceArray
  (params (Array :type Array%20of%20Static%20Material%20Structures))
  (bind _newlocalvar (LocalVariables|GetNewLocalVar))
  (for _array_element Array
    (Utilities|Array|Add _newlocalvar (.MaterialInterface (Utilities|Struct|BreakStaticMaterial _array_element))))
  (return _newlocalvar))

(fn ConvertSMtoInstanceSM
  (params (Force :type Boolean)))

(fn ConvertSMtoInstanceSM2
  (params (Force :type Boolean)))

(fn Convert
  (params (NewLocalVar_01 :type Array%20of%20Static%20Mesh%20Component%20Object%20References) (Delete :type Boolean) (Hidden :type Boolean) (IgnoreInit :type Boolean) (NewMobility :type EComponentMobility%20Enum :default "Static"))
  (bind _instancestaticmeshes (LocalVariables|GetInstanceStaticMeshes))
  (if IgnoreInit
    _
    (elif (Variables|Default|GetIsInit?)
      (return false 0)
      (else
        (Variables|Default|SetIsInit? true))))
  (bind _output_get (LocalVariables|SetInputStaticMeshesComponents NewLocalVar_01))
  (for _array_element _output_get
    (if (== (Utilities|Array|FindItem (LocalVariables|GetStaticMeshes) (Variables|/Script/Engine.StaticMeshComponent|GetStaticMesh _array_element)) -1)
      (bind _returnvalue (Utilities|Array|Add (LocalVariables|GetStaticMeshes) (Variables|/Script/Engine.StaticMeshComponent|GetStaticMesh _array_element)))
      (bind _outputpin (CallFunction|CreateInstanceStaticMesh (Variables|/Script/Engine.StaticMeshComponent|GetStaticMesh _array_element) (Rendering|Material|GetMaterials _array_element) NewMobility))
      (Utilities|Array|Add _instancestaticmeshes _outputpin))
    (Components|InstancedStaticMesh|AddInstance (Utilities|Array|Get(acopy) _instancestaticmeshes (select (== (Utilities|Array|FindItem (LocalVariables|GetStaticMeshes) (Variables|/Script/Engine.StaticMeshComponent|GetStaticMesh _array_element)) -1) _returnvalue (Utilities|Array|FindItem (LocalVariables|GetStaticMeshes) (Variables|/Script/Engine.StaticMeshComponent|GetStaticMesh _array_element)))) (Transformation|GetWorldTransform _array_element) true)
    (if Delete
      (Components|DestroyComponent _array_element)
      (elif Hidden
        (Rendering|SetVisibility _array_element false false))))
  (return true (LocalVariables|GetInstanceStaticMeshes)))

(fn CreateInstanceStaticMesh
  (params (StaticMesh :type Static%20Mesh%20Object%20Reference) (Materials :type Array%20of%20Material%20Interface%20Object%20References) (NewMobility :type EComponentMobility%20Enum :default "Static"))
  (bind _returnvalue (Components|GetOwner))
  (bind _returnvalue_2 (Game|AddComponentbyClass _returnvalue "/Script/Engine.InstancedStaticMeshComponent" true (Math|Transform|MakeTransform "0, 0, 0")))
  (bind _returnvalue_3 (Transformation|AttachComponentToComponent _returnvalue_2 (Variables|/Script/Engine.Actor|GetRootComponent _returnvalue) "None" "SnapToTarget" "SnapToTarget" "KeepWorld" true))
  (if _returnvalue_3
    (bind _returnvalue_4 (Components|StaticMesh|SetStaticMesh _returnvalue_2 StaticMesh))
    (if _returnvalue_4
      (for (_array_element _array_index) Materials
        (Rendering|Material|SetMaterial _returnvalue_2 _array_index _array_element))
      (Transformation|SetMobility _returnvalue_2 NewMobility)
      (return _returnvalue_2))))

(fn Setup
  (Base|Convert (Actor|GetComponentsByClass (Components|GetOwner) "/Script/Engine.StaticMeshComponent") true false false "Static"))