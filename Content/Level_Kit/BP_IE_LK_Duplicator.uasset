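; Level-kit Blueprint that duplicates the instanced static meshes of a referenced actor onto itself.
; DuplicateInstanceMeshes matches the source root's mobility, then creates an InstancedStaticMeshComponent per source component, snapped to its own root.
; Each receives the source mesh and local-space instance transforms; materials are written to the mesh asset, so component overrides are not copied.
; The construction script's Refresh-driven call is disconnected, so nothing here triggers duplication automatically.
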(event EventBeginPlay)

(event Collision|EventActorBeginOverlap
  (params (OtherActor :type Actor%20Object%20Reference)))

(event EventTick
  (params (DeltaSeconds :type Float%20%28single-precision%29)))

(fn ConstructionScript)

(fn DuplicateInstanceMeshes
  (bind _self self)
  (bind _actorref (Variables|BP_IE_LK_Duplicator_C|GetActorRef _self))
  (Utilities|IsValid (Variables|Default|GetActorRef)
    (:Is%20Valid
      (Transformation|SetMobility (Variables|/Script/Engine.Actor|GetRootComponent _self) (Variables|/Script/Engine.SceneComponent|GetMobility (Variables|/Script/Engine.Actor|GetRootComponent _actorref)))
      (for _array_element (Actor|GetComponentsByClass _actorref "/Script/Engine.InstancedStaticMeshComponent")
        (bind _returnvalue (Game|AddComponentbyClass _self "/Script/Engine.InstancedStaticMeshComponent" true (Transformation|GetRelativeTransform _array_element)))
        (Transformation|SetMobility _returnvalue (Variables|/Script/Engine.SceneComponent|GetMobility _array_element))
        (bind _returnvalue_2 (Transformation|AttachComponentToComponent _returnvalue (Variables|/Script/Engine.Actor|GetRootComponent _self) "None" "SnapToTarget" "SnapToTarget" "KeepWorld" true))
        (if _returnvalue_2
          (Utilities|FlowControl|Sequence
            (:then_0
              (Components|StaticMesh|SetStaticMesh _returnvalue (Variables|/Script/Engine.StaticMeshComponent|GetStaticMesh _array_element))
              (Variables|/Script/Engine.StaticMesh|SetStaticMaterials (Variables|/Script/Engine.StaticMeshComponent|GetStaticMesh _returnvalue) (Variables|/Script/Engine.StaticMesh|GetStaticMaterials (Variables|/Script/Engine.StaticMeshComponent|GetStaticMesh _array_element)))
              (for _index (range 0 (- (Components|InstancedStaticMesh|GetInstanceCount _array_element) 1))
                (Components|InstancedStaticMesh|AddInstance _returnvalue (.OutInstanceTransform (Components|InstancedStaticMesh|GetInstanceTransform _array_element _index false)) false)))))))))