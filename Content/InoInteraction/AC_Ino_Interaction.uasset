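; Interaction component that detects objects under the camera and relays hover and press input to them.
; CheckInteraction sphere-traces along the camera's forward vector, broadcasts the hit through OnInteraction and tracks actors tagged "InoInt".
; It sends InoBridgeMessage on every tagged hit and when clearing the hovered actor, but not when switching directly between tagged actors.
; Interact forwards press and release to the hovered actor with the stored hit.
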(event Custom|Interact
  (params (Pressed :type Boolean))
  (bind _currenthoveredactor (Variables|Default|GetCurrentHoveredActor))
  ;[1 1 1] Comment
  (Utilities|IsValid _currenthoveredactor
    (:Is%20Valid
      (Class|IntIEInoBridge|InoBridge(Message) _currenthoveredactor self 0 "(TagName=\"Ino.Bridge.Int\")" (select Pressed "NewEnumerator2" "NewEnumerator3") "NewEnumerator0" false 0 0 "" 0 (Variables|Default|GetCurrentHitResult)))))

(event Custom|CheckInteraction
  (params (TraceDistance :type Integer) (Radius :type Float%20%28single-precision%29))
  (bind _returnvalue (Game|GetPlayerCameraManager 0))
  (bind _rootcomponent (Variables|/Script/Engine.Actor|GetRootComponent _returnvalue))
  (bind _returnvalue_2 (Transformation|GetWorldLocation _rootcomponent))
  ;[1 1 1] Comment
  (bind (_outhit _returnvalue_3) (Collision|SphereTraceByChannel _returnvalue_2 (+ (* (Math|Vector|GetForwardVector _rootcomponent) TraceDistance) _returnvalue_2) Radius "TraceTypeQuery1" false 0 (select (.bActive (Utilities|Struct|BreakInoLogPreset (Variables|Default|GetInoLogPreset))) "ForDuration" "None") true "(R=1.000000,G=0.000000,B=0.000000,A=1.000000)" "(R=0.000000,G=1.000000,B=0.000000,A=1.000000)" 0.03))
  (Variables|Default|SetCurrentHit _returnvalue_3)
  (Default|CallOnInteraction _returnvalue_3 _outhit)
  (if _returnvalue_3
    (Variables|Default|SetCurrentHitResult _outhit)
    (if (!= (Utilities|Array|FindItem (Variables|/Script/Engine.Actor|GetTags (.HitActor (Collision|BreakHitResult _outhit))) "InoInt") -1)
      (bind _output_get (Variables|Default|SetCurrentHoveredActor (.HitActor (Collision|BreakHitResult _outhit))))
      (Class|IntIEInoBridge|InoBridge(Message) _output_get self 0 "(TagName=\"Ino.Bridge.Int\")" "NewEnumerator5" "NewEnumerator0" false 0 0 "" 0 (Variables|Default|GetCurrentHitResult))
      (else
        (Utilities|IsValid (Variables|Default|GetCurrentHoveredActor) :!label _label
          (:Is%20Valid
            (Class|IntIEInoBridge|InoBridge(Message) (Variables|Default|GetCurrentHoveredActor) self 0 "(TagName=\"Ino.Bridge.Int\")" "NewEnumerator6" "NewEnumerator0" false 0 0 "" 0 (Variables|Default|GetCurrentHitResult))
            (Variables|Default|SetCurrentHoveredActor 0)))))
    (else
      (goto _label))))