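; BP_Ino_Interaction detects the interactable actor in front of the player camera and relays hover and interact input to it.
; CheckInteraction sphere-traces forward on Visibility, caching a hit actor tagged "InoInt" as hovered, or clearing it otherwise.
; Interact forwards press and release to that cached actor.
; All notifications go through InoBridgeMessage with the Ino.Bridge.Int tag and an enum type, keeping targets decoupled.
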(event Custom|Interact
  (params (Pressed :type Boolean))
  (bind _currenthoveredactor (Variables|Default|GetCurrentHoveredActor))
  (Utilities|IsValid _currenthoveredactor
    (:Is%20Valid
      (Class|IntIEInoBridge|InoBridge(Message) _currenthoveredactor self 0 "(TagName=\"Ino.Bridge.Int\")" (select Pressed "NewEnumerator2" "NewEnumerator3") "NewEnumerator0" false))))

(event Custom|CheckInteraction
  (params (TraceDistance :type Integer) (Radius :type Float%20%28single-precision%29))
  (bind _returnvalue (Game|GetPlayerCameraManager 0))
  (bind _rootcomponent (Variables|/Script/Engine.Actor|GetRootComponent _returnvalue))
  (bind _returnvalue_2 (Transformation|GetWorldLocation _rootcomponent))
  (bind (_outhit _returnvalue_3) (Collision|SphereTraceByChannel _returnvalue_2 (+ (* (Math|Vector|GetForwardVector _rootcomponent) TraceDistance) _returnvalue_2) Radius "TraceTypeQuery1" false 0 (select (Variables|AConfig|GetDebug) "ForDuration" "None") true "(R=1.000000,G=0.000000,B=0.000000,A=1.000000)" "(R=0.000000,G=1.000000,B=0.000000,A=1.000000)" 0.03))
  (if _returnvalue_3
    (if (!= (Utilities|Array|FindItem (Variables|/Script/Engine.Actor|GetTags (.HitActor (Collision|BreakHitResult _outhit))) "InoInt") -1)
      (bind _output_get (Variables|Default|SetCurrentHoveredActor (.HitActor (Collision|BreakHitResult _outhit))))
      (Class|IntIEInoBridge|InoBridge(Message) _output_get self 0 "(TagName=\"Ino.Bridge.Int\")" "NewEnumerator5" "NewEnumerator0" false 0 0 "" _outhit)
      (else
        (Utilities|IsValid (Variables|Default|GetCurrentHoveredActor) :!label _label
          (:Is%20Valid
            (Class|IntIEInoBridge|InoBridge(Message) (Variables|Default|GetCurrentHoveredActor) self 0 "(TagName=\"Ino.Bridge.Int\")" "NewEnumerator6" "NewEnumerator0" false)
            (Variables|Default|SetCurrentHoveredActor 0)))))
    (else
      (goto _label))))