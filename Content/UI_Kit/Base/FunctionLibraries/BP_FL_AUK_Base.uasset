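; Base Blueprint function library for the AUK UI Kit, with pure-style helpers that restyle brushes, buttons and fonts.
; Brush, button and font helpers rebuild structs, treating transparent magenta, -1 or invalid sounds as "keep original".
; Outline width is the exception: its -1 check tests the input brush instead of the override.
; Small utilities resolve color and material overrides, detect empty or "None" text, and map platform name to an enum.
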(fn AUKSetSlateBrushColor
  (params (InputSlateBrush :type Slate%20Brush%20Structure%20%28by%20ref%29) (Tint%20Color :type Linear%20Color%20Structure :default "(R=1.000000,G=0.000000,B=1.000000,A=0.000000)") (OutlineColor :type Linear%20Color%20Structure :default "(R=1.000000,G=0.000000,B=1.000000,A=0.000000)") (OutlineRadius :type Vector%204%20Structure) (OutlineWidth :type Float%20%28double-precision%29))
  (bind (_drawas _tiling _mirroring _imagesize _margin _tintcolor _outlinesettings _resourceobject) (Utilities|Struct|BreakSlateBrush InputSlateBrush))
  (bind (_x _y _z _w) (Math|Vector4|BreakVector4 OutlineRadius))
  (bind (_specifiedcolor _coloruserule) (Utilities|Struct|BreakSlateColor _tintcolor))
  (bind (_cornerradii _color _width _roundingtype _busebrushtransparency) (Utilities|Struct|BreakSlateBrushOutlineSettings _outlinesettings))
  (bind (_specifiedcolor_2 _coloruserule_2) (Utilities|Struct|BreakSlateColor _color))
  (bind (_x_2 _y_2 _z_2 _w_2) (Math|Vector4|BreakVector4 _cornerradii))
  (return (Utilities|Struct|MakeSlateBrush _drawas _tiling _mirroring _imagesize _margin (Utilities|Struct|MakeSlateColor (select (== Tint%20Color "(R=1.000000,G=0.000000,B=1.000000,A=0.000000)") _specifiedcolor Tint%20Color) _coloruserule) (Utilities|Struct|MakeSlateBrushOutlineSettings (Math|Vector4|MakeVector4 (select (== _x -1.0) _x_2 _x) (select (== _y -1.0) _y_2 _y) (select (== _z -1.0) _z_2 _z) (select (== _w -1.0) _w_2 _w)) (Utilities|Struct|MakeSlateColor (select (== OutlineColor "(R=1.000000,G=0.000000,B=1.000000,A=0.000000)") _specifiedcolor_2 OutlineColor) _coloruserule_2) (select (== _width -1.0) _width OutlineWidth) _roundingtype _busebrushtransparency) _resourceobject)))

(fn AUKButtonSetStyleColorandSound
  (params (InputButtonStyle :type Button%20Style%20Structure%20%28by%20ref%29) (TintColor :type ST%20AUK%20Button%20Color%20Structure) (OutlineColor :type ST%20AUK%20Button%20Color%20Structure) (PressedSound :type Object%20Object%20Reference) (HoveredSound :type Object%20Object%20Reference) (CornerRadius :type ST%20AUK%20Outline%20Settings%20Structure))
  (bind (_normal _hovered _pressed _disabled _normalforeground _hoveredforeground _pressedforeground _disabledforeground _normalpadding _pressedpadding _pressedslatesound _hoveredslatesound) (Utilities|Struct|BreakButtonStyle InputButtonStyle))
  (bind (_normal_2 _hovered_2 _pressed_2 _disabled_2) (Utilities|Struct|BreakST_AUK_ButtonColor OutlineColor))
  (bind (_normal_3 _hovered_3 _pressed_3 _disabled_3) (Utilities|Struct|BreakST_AUK_ButtonColor TintColor))
  (bind (_normalradious _normalwidth _hoveredradious _hoveredwidth _pressedradious _pressedwidth _disabledradious _disabledwidth) (Utilities|Struct|BreakST_AUK_OutlineSettings CornerRadius))
  (return (Utilities|Struct|MakeButtonStyle (AUK|AUKSetSlateBrushColor _normal _normal_3 _normal_2 _normalradious _normalwidth) (AUK|AUKSetSlateBrushColor _hovered _hovered_3 _hovered_2 _hoveredradious _hoveredwidth) (AUK|AUKSetSlateBrushColor _pressed _pressed_3 _pressed_2 _pressedradious _pressedwidth) (AUK|AUKSetSlateBrushColor _disabled _disabled_3 _disabled_2 _disabledradious _disabledwidth) _normalforeground _hoveredforeground _pressedforeground _disabledforeground _normalpadding _pressedpadding (Utilities|Struct|MakeSlateSound (select (Utilities|IsValid PressedSound) PressedSound (Utilities|Struct|BreakSlateSound _pressedslatesound))) (Utilities|Struct|MakeSlateSound (select (Utilities|IsValid HoveredSound) HoveredSound (Utilities|Struct|BreakSlateSound _hoveredslatesound))))))

(fn AUKTextBoxSetFont
  (params (InFontInfo :type Slate%20Font%20Info%20Structure) (Size :type Integer) (TypeFace :type E_AUK_TypeFace%20Enum :default "NewEnumerator0"))
  (bind (_fontobject _fontmaterial _outlinesettings _typefacefontname _size _letterspacing _skewamount) (Utilities|Struct|BreakSlateFontInfo InFontInfo))
  (return (Utilities|Struct|MakeSlateFontInfo _fontobject _fontmaterial _outlinesettings (Utilities|String|StringToName (Utilities|String|EnumtoString TypeFace)) (select (== Size -1) _size Size) _letterspacing _skewamount)))

(fn AUKIsColorChanged?
  (params (DefaultColor :type Linear%20Color%20Structure) (ChangedColor :type Linear%20Color%20Structure))
  (return (select (== (.A (Utilities|Struct|BreakLinearColor ChangedColor)) 0.0) DefaultColor ChangedColor)))

(fn AUKIsTextEmpty?
  (params (Text :type Text%20%28by%20ref%29))
  (return (or (Utilities|Enum|Equal(Enum) Text (Utilities|Text|MakeLiteralText "None")) (Utilities|Enum|Equal(Enum) Text (Utilities|Text|MakeLiteralText "")))))

(fn AUKIsMaterialChanged?
  (params (DefaultMaterial :type Material%20Instance%20Object%20Reference) (ChangedMaterial :type Material%20Instance%20Object%20Reference))
  (return (select (Utilities|IsValid ChangedMaterial) ChangedMaterial DefaultMaterial)))

(fn AUKGetPlatform
  (switch string (Game|GetPlatformName)
    (:Default
      (return "NewEnumerator0"))
    (:windows
      (return "NewEnumerator0"))
    (:mac
      (return "NewEnumerator3"))
    (:linux
      (return "NewEnumerator2"))
    (:ios
      (return "NewEnumerator4"))
    (:android
      (return "NewEnumerator1"))))