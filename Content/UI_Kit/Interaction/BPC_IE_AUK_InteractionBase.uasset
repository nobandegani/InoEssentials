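; Base interaction component that tracks actors overlapping a supplied detection mesh, highlights the nearest eligible one and sends interactions to it.
; Init stores the mesh, scene components and ALS camera, detaches the cone's scene component for external transform updates, and binds overlap events.
; Overlaps and character updates trigger nearest-actor selection, notifying other overlapping actors separately.
; All communication uses generic InoBridge messages with gameplay tags, with a JSON flag triggering re-highlighting.
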(event OnComponentEndOverlap(SM_Int)
  (params (OverlappedComponent :type Primitive%20Component%20Object%20Reference) (OtherActor :type Actor%20Object%20Reference) (OtherComp :type Primitive%20Component%20Object%20Reference) (OtherBodyIndex :type Integer))
  ;[1 1 1] EndOverlap
)

(event OnComponentBeginOverlap(SM_Int)
  (params (OverlappedComponent :type Primitive%20Component%20Object%20Reference) (OtherActor :type Actor%20Object%20Reference) (OtherComp :type Primitive%20Component%20Object%20Reference) (OtherBodyIndex :type Integer) (bFromSweep :type Boolean) (SweepResult :type Hit%20Result%20Structure%20%28by%20ref%29))
  ;[1 1 1] BeginOverlap
)

(event Custom|CustomEvent
  (bind _sm_int (Variables|Default|GetSM_Int))
  (Collision|AssignOnComponentBeginOverlap _sm_int (delegate Custom|OnComponentBeginOverlap_Event))
  (Collision|AssignOnComponentEndOverlap _sm_int (delegate Custom|OnComponentEndOverlap_Event)))

(event Custom|UpdateInteractionConeTransform
  (params (NewTransform :type Transform%20%28by%20ref%29))
  ;[1 1 1] UpdateInteractionConeTransform
  (Transformation|SetWorldTransform (Variables|Default|GetScn_Int) NewTransform false false))

(event Custom|OnComponentBeginOverlap_Event
  (params (OverlappedComponent :type Primitive%20Component%20Object%20Reference) (OtherActor :type Actor%20Object%20Reference) (OtherComp :type Primitive%20Component%20Object%20Reference) (OtherBodyIndex :type Integer) (bFromSweep :type Boolean) (SweepResult :type Hit%20Result%20Structure%20%28by%20ref%29))
  (bind _outjsonstring (Utilities|JsontoStringwithVar "HighlightNearby" (Class|KismetSystemLibrary|MakeLiteralBool true) false)
    (:Return
      (CallFunction|InoBridge OtherActor 0 "(TagName=\"InterActionType\")" "NewEnumerator5" "NewEnumerator0" true 0 _outjsonstring))))

(event Custom|Interact
  (bind _highlightedactor (Variables|Default|GetHighlightedActor))
  ;[1 1 1] Interact
  (Utilities|IsValid _highlightedactor
    (:Is%20Valid
      (Class|IntIEInoBridge|InoBridge(Message) :self _highlightedactor :Caller self :Index 99 :Type "NewEnumerator2" :GamePlayTag (Variables|AConfig|GetCurrentMode)))))

(event Custom|OnComponentEndOverlap_Event
  (params (OverlappedComponent :type Primitive%20Component%20Object%20Reference) (OtherActor :type Actor%20Object%20Reference) (OtherComp :type Primitive%20Component%20Object%20Reference) (OtherBodyIndex :type Integer))
  (CallFunction|InoBridge OtherActor 0 "(TagName=\"InterActionType\")" "NewEnumerator6" "NewEnumerator0" false))

(event Custom|CharacterUpdated
  (CallFunction|HighlightNear))

(event Custom|HighlightNear
  ;[1 1 1] HighlightNear
  (bind _returnvalue (CallFunction|FindNearestInter))
  (Utilities|IsValid _returnvalue
    (:Is%20Valid
      (Variables|Default|SetHighlightedActor _returnvalue)
      (CallFunction|InoBridge _returnvalue 0 "(TagName=\"InterActionType\")" "NewEnumerator4" "NewEnumerator0" false)
      (CallFunction|FindOthers _returnvalue))
    (:Is%20Not%20Valid
      (Variables|Default|SetHighlightedActor 0))))

(event EventBeginPlay)

(fn FindNearestInter
  (bind _sm_int (Variables|Default|GetSM_Int))
  (bind _overlappingactors (Collision|GetOverlappingActors _sm_int "/Script/Engine.Actor" :!class /Script/Engine.PrimitiveComponent))
  (for (_array_element _array_index) _overlappingactors
    (bind _o_bool (Class|IntIEInoBridge|InoBridge(Message) :self _array_element :Caller self :Index 99 :GamePlayTag "(TagName=\"InteractionType.Normal\")"))
    (if _o_bool
      (if (< (Math|Vector|Distance(Vector) (Transformation|GetActorLocation _array_element) (Transformation|GetActorLocation (Components|GetOwner))) (LocalVariables|GetNewLocalVar))
        (LocalVariables|SetNewLocalVar (Math|Vector|Distance(Vector) (Transformation|GetActorLocation _array_element) (Transformation|GetActorLocation (Components|GetOwner))))
        (LocalVariables|SetNewLocalVar_0 _array_index))))
  (if (Utilities|Array|IsValidIndex _overlappingactors (LocalVariables|GetNewLocalVar_0))
    (return (LocalVariables|GetNewLocalVar_0) (Utilities|Array|Get(acopy) _overlappingactors (LocalVariables|GetNewLocalVar_0)))
    (else
      (return -1 0))))

(fn FindOthers
  (params (NewParam :type Actor%20Object%20Reference))
  (for _array_element (Collision|GetOverlappingActors (Variables|Default|GetSM_Int) "/Script/Engine.Actor" :!class /Script/Engine.PrimitiveComponent)
    (if (not (== NewParam _array_element))
      (Class|IntIEInoBridge|InoBridge(Message) :self _array_element :Caller self :Index 99 :Type "NewEnumerator7" :GamePlayTag "(TagName=\"InterActionType\")")))
  (return))

(fn Init
  (params (Scn_Int :type Scene%20Component%20Object%20Reference) (SM_Int :type Static%20Mesh%20Component%20Object%20Reference) (Scn_EndInt :type Scene%20Component%20Object%20Reference) (ALSCamera :type Als%20Camera%20Component%20Object%20Reference))
  (Variables|Default|SetScn_Int Scn_Int)
  (Variables|Default|SetSM_Int SM_Int)
  (Variables|Default|SetScn_EndInt Scn_EndInt)
  (Transformation|DetachFromComponent (Variables|Default|GetScn_Int) "KeepRelative" "KeepRelative" "KeepRelative" true)
  (CallFunction|CustomEvent)
  (Variables|Default|SetALSCamera ALSCamera))

(fn InoBridge
  (params (Caller :type Object%20Object%20Reference) (Index :type Integer) (Tag :type Gameplay%20Tag%20Structure) (Type :type E_IE_IB_InteractionType%20Enum :default "NewEnumerator0") (Replication :type E_IE_IB_Replication%20Enum :default "NewEnumerator0") (Relaible :type Boolean) (BoolPass :type Boolean) (IntPass :type Integer) (ObjectPass :type Object%20Object%20Reference) (StringPass :type String) (GamePlayTag :type Gameplay%20Tag%20Structure) (Relaible? :type Boolean))
  (bind _outjsonobject (Class|JsonBlueprintFunctionLibrary|FromString StringPass))
  (Utilities|FlowControl|Sequence
    (:then_0
      (Class|IntIEInoBridge|InoBridge(Message) :self Caller :Caller self :Index 99 :Type Type :Replication Replication :ObjectPass ObjectPass :StringPass (Utilities|String|ToString(Float) (Math|Vector|Distance(Vector) (Transformation|GetWorldLocation (Variables|Default|GetScn_EndInt)) (Transformation|GetWorldLocation (Variables|Default|GetSM_Int)))) :GamePlayTag (Variables|AConfig|GetCurrentMode) :Relaible? Relaible?))
    (:then_1
      (bind _outvalue (|GetJsonField _outjsonobject "HighlightNearby"))
      (if _outvalue
        (CallFunction|HighlightNear)))))