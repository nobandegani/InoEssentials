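; Interaction indicator actor from the UI kit that shows a WBP_AUK_IS_Main widget for an interactable actor.
; InoBridge messages at index 99 set the target actor and range, load a config by gameplay tag, and drive hover, highlight, press and release.
; While active, Tick optionally scales the widget, toggles usability by player distance, and smoothly yaws toward the player.
; Construction applies a test config for preview.
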(event Custom|ControlActivity
  (params (Enable? :type Boolean) (DeleteRef :type Boolean))
  (bind _maxdistance (Variables|Base|GetMaxDistance))
  ;[1 1 1] ControlActivity
  (Variables|Base|SetEnableHighlight Enable?)
  (Actor|Tick|SetActorTickEnabled Enable?)
  (Rendering|SetActorHiddenInGame (not Enable?))
  (Utilities|FlowControl|Sequence
    (:then_0
      (if DeleteRef
        (Variables|Base|SetActorRef 0)))
    (:then_1
      ;[1 1 1] UpdateTextVisibilityOnDIstance
      (Utilities|FlowControl|DoOnce false) ; enters at Reset
    )))

(event Custom|Use
  (params (Tag :type Gameplay%20Tag%20Structure))
  ;[1 1 1] Use
  (CallFunction|ControlActivity false false)
  (Variables|Base|SetUsed? true)
  (Default|CallOnUse Tag))

(event Custom|UpdateSetup
  (params (UpdateSetup :type ST%20AUK%20IS%20UI%20Config%20Structure))
  (bind _ui_ref (Variables|Base|GetUI%20Ref))
  ;[1 1 1] UpdateSetup
  (bind _output_get (Variables|Base|SetCurrent%20Config UpdateSetup))
  (Utilities|IsValid _ui_ref
    (:Is%20Valid
      (Default|SetupIntMain _ui_ref _output_get)
      ;;[1 1 1] Comment
      (Utilities|FlowControl|Sequence
        (:then_0
          (if (not (.ScaleOnDistance (Utilities|Struct|BreakST_AUK_IS_UIConfig (Variables|Base|GetCurrent%20Config))))
            (Default|UpdateScale (Variables|Base|GetUI%20Ref) 1.0)))
        (:then_1
          (if (not (.UsableOnDistance (Utilities|Struct|BreakST_AUK_IS_UIConfig (Variables|Base|GetCurrent%20Config))))
            (Variables|Base|SetIsUsable? true)
            (Default|ToggleInt (Variables|Base|GetUI%20Ref) true)))))))

(event Custom|UnUse
  ;[1 1 1] UnUse
  (Utilities|IsValid (Variables|Base|GetActorRef)
    (:Is%20Valid
      (Variables|Base|SetUsed? false)
      (CallFunction|ControlActivity true false))))

(event Custom|Highlight
  (if (Variables|Base|GetIsUsable?)
    (Default|Highlight (Variables|Base|GetUI%20Ref) true)))

(event Custom|UnHighlight
  (Default|Highlight (Variables|Base|GetUI%20Ref) false))

(event Custom|TestUpdate
  (params (TestConfig :type ST%20AUK%20IS%20UI%20Config%20Structure) (TestScale :type Float%20%28double-precision%29))
  ;[1 1 1] TestUpdate
  (Variables|ATest|SetTestScale TestScale)
  (Variables|ATest|SetTestConfig TestConfig)
  (bind _aswbp_auk_is_main (Utilities|Casting|CastToWBP_AUK_IS_Main (UserInterface|GetWidget (Variables|Default|GetWidget))))
  (Default|SetupIntMain _aswbp_auk_is_main (Variables|ATest|GetTestConfig))
  (Default|UpdateScale _aswbp_auk_is_main (Variables|ATest|GetTestScale)))

(event Custom|UpdateConstruction
  (CallFunction|TestUpdate (Variables|ATest|GetTestConfig) (Variables|ATest|GetTestScale)))

(event EventBeginPlay
  ;[1 1 1] Beginplay
  (bind _aswbp_auk_is_main (Utilities|Casting|CastToWBP_AUK_IS_Main (UserInterface|GetWidget (Variables|Default|GetWidget))))
  (Variables|Base|SetUI%20Ref _aswbp_auk_is_main)
  (CallFunction|ControlActivity false false))

(event EventTick
  (params (DeltaSeconds :type Float%20%28single-precision%29))
  (bind _maxdistance (Variables|Base|GetMaxDistance))
  (if (Variables|Base|GetEnableHighlight)
    (Utilities|FlowControl|Sequence
      (:then_0
        (Utilities|FlowControl|Sequence
          (:then_0
            (Variables|Base|SetCurrentDistance (Math|Vector|Distance(Vector) (Transformation|GetActorLocation (Variables|Base|GetActorRef)) (Transformation|GetActorLocation (Game|Player|GetPlayerPawn 0))))
            ;[1 1 1] UpdateScaleOnDIstance
            (if (.ScaleOnDistance (Utilities|Struct|BreakST_AUK_IS_UIConfig (Variables|Base|GetCurrent%20Config)))
              (Default|UpdateScale (Variables|Base|GetUI%20Ref) (Math|Float|MapRangeClamped (Variables|Base|GetCurrentDistance) (Variables|Base|GetMaxDistance) 5e+01 0.1 1.0))))
          (:then_1
            ;[1 1 1] UpdateTextVisibilityOnDIstance
            (if (.UsableOnDistance (Utilities|Struct|BreakST_AUK_IS_UIConfig (Variables|Base|GetCurrent%20Config)))
              (Utilities|FlowControl|Sequence
                (:then_0
                  (Utilities|FlowControl|DoOnce false
                    (:Completed
                      (bind _output_get (Variables|Base|SetIsUsable? (< (Variables|Base|GetCurrentDistance) (- _maxdistance (* _maxdistance (.DistanceToActive (Utilities|Struct|BreakST_AUK_IS_UIConfig (Variables|Base|GetCurrent%20Config)))))) :!label _label))
                      (Default|ToggleInt (Variables|Base|GetUI%20Ref) _output_get)
                      (if (not _output_get)
                        (CallFunction|UnHighlight)))))
                (:then_1
                  (if (not (== (< (Variables|Base|GetCurrentDistance) (- _maxdistance (* _maxdistance (.DistanceToActive (Utilities|Struct|BreakST_AUK_IS_UIConfig (Variables|Base|GetCurrent%20Config)))))) (Variables|Base|GetIsUsable?)))
                    (goto _label))))))))
      (:then_1
        ;[1 1 1] set the rotaiton
        (if (.FaceToActor (Utilities|Struct|BreakST_AUK_IS_UIConfig (Variables|Base|GetCurrent%20Config)))
          (Transformation|SetActorRotation (Math|Rotator|MakeRotator 0.0 0.0 (Math|Interpolation|FInterpTo (.Yaw (Math|Rotator|BreakRotator (Transformation|GetActorRotation))) (.Yaw (Math|Rotator|BreakRotator (Math|Rotator|FindLookatRotation (Transformation|GetActorLocation) (Transformation|GetActorLocation (Game|Player|GetPlayerPawn 0))))) DeltaSeconds 5.0))))))))

(fn ConstructionScript
  (CallFunction|UpdateConstruction))

(fn InoBridge
  (params (Caller :type Object%20Object%20Reference) (Index :type Integer) (Tag :type Gameplay%20Tag%20Structure) (Type :type E_IE_IB_InteractionType%20Enum :default "NewEnumerator0") (Replication :type E_IE_IB_Replication%20Enum :default "NewEnumerator0") (Relaible :type Boolean) (BoolPass :type Boolean) (IntPass :type Integer) (ObjectPass :type Object%20Object%20Reference) (StringPass :type String) (GamePlayTag :type Gameplay%20Tag%20Structure) (Relaible? :type Boolean))
  (bind _returnvalue (Math|Conversions|ToFloat(Integer) StringPass))
  (bind _isusable_ (Variables|Base|GetIsUsable?))
  (bind _enablehighlight (Variables|Base|GetEnableHighlight))
  (bind _uiconfigs (Variables|AConfig|GetUiConfigs))
  (bind _current_config (Variables|Base|GetCurrent%20Config))
  (bind _used_ (Variables|Base|GetUsed?))
  (bind _usableondistance (Utilities|Struct|BreakST_AUK_IS_UIConfig _current_config))
  (bind (_value _returnvalue_2) (Utilities|Map|Find _uiconfigs GamePlayTag))
  (bind _returnvalue_3 (not _used_))
  (bind _returnvalue_4 (not _usableondistance))
  (bind _returnvalue_5 (or _returnvalue_3 false))
  (bind _returnvalue_6 (or _returnvalue_4 _isusable_))
  (bind _returnvalue_7 (Math|Boolean|ANDBoolean _enablehighlight _returnvalue_6 _returnvalue_5))
  (if (== Index 99)
    (bind _asactor (Utilities|Casting|CastToActor Caller))
    (if (== _asactor (Variables|Base|GetActorRef))
      _
      (else
        (Variables|Base|SetActorRef _asactor)))
    (if (== _returnvalue 0.0)
      _
      (else
        (Variables|Base|SetMaxDistance _returnvalue)))
    (if Relaible?
      (if _returnvalue_2
        (CallFunction|UpdateSetup _value)
        (if (.Activate? (Utilities|Struct|BreakST_AUK_IS_UIConfig (Variables|Base|GetCurrent%20Config))) :!label _label
          (Utilities|FlowControl|Sequence
            (:then_0
              (switch Utilities|FlowControl|Switch|SwitchonE_IE_IB_InteractionType Type
                (:NewEnumerator4
                  (CallFunction|Highlight))
                (:NewEnumerator7
                  (CallFunction|UnHighlight))
                (:NewEnumerator2
                  (if _returnvalue_7
                    (CallFunction|Use GamePlayTag)))
                (:NewEnumerator3
                  (if (Variables|Base|GetUsed?)
                    (CallFunction|UnUse)))
                (:NewEnumerator5
                  (if (not (Variables|Base|GetUsed?))
                    (CallFunction|ControlActivity true false)))
                (:NewEnumerator6
                  (CallFunction|ControlActivity false true))))
            (:then_1
              (return 0 0 GamePlayTag "NewEnumerator0" "NewEnumerator0" false false 0 0 "" Index _returnvalue_7)))))
      (else
        (goto _label)))))