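; Tooltip component that shows a screen-space text widget on its owner while a character is in range.
; On BeginPlay it adds and attaches a widget component holding WBP_AUK_ToolTip_BaseTemplate, initially hidden, plus a pawn-overlap sphere of configurable radius, visible for debugging.
; Sphere begin and end overlaps toggle widget visibility, but only for actors whose class is exactly Character, so subclasses do not trigger it.
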(event Custom|OnComponentBeginOverlap_Event
  (params (OverlappedComponent :type Primitive%20Component%20Object%20Reference) (OtherActor :type Actor%20Object%20Reference) (OtherComp :type Primitive%20Component%20Object%20Reference) (OtherBodyIndex :type Integer) (bFromSweep :type Boolean) (SweepResult :type Hit%20Result%20Structure%20%28by%20ref%29))
  ;[1 1 1] Comment
  (if (== (Utilities|GetClass OtherActor) (Variables|Config|GetCharacter))
    (CallFunction|CustomEvent false)))

(event Custom|OnComponentEndOverlap_Event
  (params (OverlappedComponent :type Primitive%20Component%20Object%20Reference) (OtherActor :type Actor%20Object%20Reference) (OtherComp :type Primitive%20Component%20Object%20Reference) (OtherBodyIndex :type Integer))
  ;[1 1 1] Comment
  (if (== (Utilities|GetClass OtherActor) (Variables|Config|GetCharacter))
    (CallFunction|CustomEvent true)))

(event Custom|CustomEvent
  (params (Hide? :type Boolean))
  ;[1 1 1] Comment
  (Rendering|SetVisibility (Variables|Default|Get3DWidgetRef) (not Hide?) false))

(event EventBeginPlay
  (Utilities|FlowControl|Sequence
    (:then_0
      ;[1 1 1] Comment
      (bind _returnvalue (Game|AddComponentbyClass (Components|GetOwner) "/Script/UMG.WidgetComponent" true (Math|Transform|MakeTransform "0, 0, 0" "0, 0, 0" (Math|Conversions|ToVector(Float) (Variables|Default|GetDrawScale)))))
      (bind _output_get (Variables|Default|Set3DWidgetRef _returnvalue))
      (Transformation|AttachComponentToComponent _output_get self "None" "SnapToTarget" "SnapToTarget" "KeepWorld" true)
      (Class|WidgetComponent|SetWidgetSpace (Variables|Default|Get3DWidgetRef) "Screen")
      (Class|WidgetComponent|SetPivot (Variables|Default|Get3DWidgetRef) (Math|Vector2D|MakeVector2D 0.5 0.1))
      (Class|WidgetComponent|SetDrawSize (Variables|Default|Get3DWidgetRef) (Variables|Config|GetDrawSize))
      (bind _returnvalue_2 (UserInterface|CreateWidget "/InoEssentials/UI_Kit/TooltipSystem/WBP_AUK_ToolTip_BaseTemplate.WBP_AUK_ToolTip_BaseTemplate_C" 0 (Variables|Config|GetTooltipText2)))
      (bind _output_get_2 (Variables|Components|SetTooltipWidgetRef _returnvalue_2))
      (UserInterface|SetWidget (Variables|Default|Get3DWidgetRef) _output_get_2)
      (CallFunction|CustomEvent true)
      (Collision|SetCollisionEnabled (Variables|Default|Get3DWidgetRef) "NoCollision"))
    (:then_1
      ;[1 1 1] Comment
      (bind _returnvalue_3 (Game|AddComponentbyClass (Components|GetOwner) "/Script/Engine.SphereComponent" true (Math|Transform|MakeTransform "0, 0, 0")))
      (bind _output_get_3 (Variables|Default|SetSphereColisionRef _returnvalue_3))
      (Transformation|AttachComponentToComponent _output_get_3 self "None" "SnapToTarget" "SnapToTarget" "KeepWorld" true)
      (Collision|AssignOnComponentBeginOverlap (Variables|Default|GetSphereColisionRef) (delegate Custom|OnComponentBeginOverlap_Event))
      (Collision|SetCollisionProfileName (Variables|Default|GetSphereColisionRef) "OverlapOnlyPawn" true :!class /Script/Engine.PrimitiveComponent)
      (Collision|AssignOnComponentEndOverlap (Variables|Default|GetSphereColisionRef) (delegate Custom|OnComponentEndOverlap_Event))
      (Components|Sphere|SetSphereRadius (Variables|Default|GetSphereColisionRef) (Variables|Config|GetIn%20Sphere%20Radius) true))
    (:then_2
      ;[1 1 1] Comment
      (Development|SetHiddeninGame (Variables|Default|GetSphereColisionRef) (not (Variables|Config|GetDebug)) false))))