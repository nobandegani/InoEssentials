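; Blueprint function library of replication debug helpers that build strings for logging and printing in multiplayer.
; GetMPKeyForInoLog joins the world context object's name with its HasAuthority result, or "none" when it is not an Actor, giving a key that reflects network authority.
; GetStringForPrint joins input text, an object's name, "from" and the player name from player controller 0's PlayerState.
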(fn GetMPKeyforInoLog
  (bind ___worldcontext (LocalVariables|Get__WorldContext))
  (bind (_asactor _bsuccess) (Utilities|Casting|CastToActor ___worldcontext))
  (return (Utilities|String|Append (Utilities|GetObjectName ___worldcontext) "-" (Utilities|String|SelectString (Utilities|String|ToString(Boolean) (Ability|HasAuthority _asactor)) "none" _bsuccess))))

(fn GetStringforPrint
  (params (InputText :type String) (Input%20Object :type Object%20Object%20Reference))
  (return (Utilities|String|Append InputText (Utilities|GetObjectName Input%20Object) " from " (PlayerState|GetPlayerName (Variables|/Script/Engine.Controller|GetPlayerState (Game|GetPlayerController 0))))))