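; Actor component that manages the text chat UI, handling its creation, removal, incoming lines and entry into typing mode.
; It creates the chat widget once and registers it with the InoUI manager, unless chat is already on screen or blocked by other UI.
; Committed messages pass a short length check before firing OnMessageRecieved, and input config resyncs after a brief delay.
; Starting messaging switches the input config and forwards to the widget.
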(event Custom|InitTextChatUI
  ;[1 1 1] Comment
  (Class|FLBase|InoLog (Utilities|String|Append "inittext chatui started" "") "Display" true "(TagName=\"Ino\")")
  (bind _result (Default|IsonScreen (.ReturnValue (CallFunction|GetInoUI)) "TextChat"))
  (if (not _result)
    (bind _blockedbyui (Default|IsBlockedbyOtherUI (.ReturnValue (CallFunction|GetInoUI))))
    (if (not _blockedbyui)
      (Utilities|IsValid (Variables|Default|GetTextChatUiRef)
        (:Is%20Valid
          _)
        (:Is%20Not%20Valid
          ;[1 1 1] Comment
          (bind _returnvalue (UserInterface|CreateWidget "/InoEssentials/InoChat/Widgets/WB_Ino_TextChat.WB_Ino_TextChat_C" (Game|GetPlayerController 0) self))
          (bind _output_get (Variables|Default|SetTextChatUiRef _returnvalue))
          (EventDispatchers|AssignOnMessageCommited _output_get (delegate Custom|On_Message_Commited_Event))))
      ;[1 1 1] Comment
      (Default|AddUI (.ReturnValue (CallFunction|GetInoUI)) "TextChat" (Variables|Default|GetTextChatUiRef) 0 0 true false)
      (Class|FLBase|InoLog (Utilities|String|Append "inittext chatui added" "") "Success" true "(TagName=\"Ino\")"))))

(event Custom|On_Message_Commited_Event
  (params (Text :type Text))
  (bind _returnvalue (Utilities|String|ToString(Text) Text))
  (bind _returnvalue_2 (Utilities|String|Len _returnvalue))
  ;[1 1 1] Comment
  (Utilities|FlowControl|Sequence
    (:then_0
      (if (and (> _returnvalue_2 0) (< _returnvalue_2 32))
        (Default|CallOnMessageRecieved Text)))
    (:then_1
      (Utilities|FlowControl|Delay 0.05)
      (Default|SyncConfigtoLatestonScreen (.ReturnValue (CallFunction|GetInoUI))))))

(fn RemoveTextChatUI
  ;[1 1 1] RemoveTextChatUI
  (EventDispatchers|UnbindallEventsfromOnMessageCommited (Variables|Default|GetTextChatUiRef))
  (Default|RemoveUI (.ReturnValue (CallFunction|GetInoUI)) "TextChat" true false false)
  (Variables|Default|SetTextChatUiRef 0))

(fn AddChattoUI
  (params (Text :type ST%20Ino%20Text%20Chat%20Item%20Structure))
  (bind _textchatuiref (Variables|Default|GetTextChatUiRef))
  ;[1 1 1] AddChatToUI
  (Utilities|IsValid _textchatuiref
    (:Is%20Valid
      (Default|AddChattoUI _textchatuiref Text))
    (:Is%20Not%20Valid
      (Class|FLBase|InoLog "not valid" "Error" true "(TagName=\"Ino\")"))))

(fn StartMessaging
  ;[1 1 1] Start messaging
  (Utilities|IsValid (Variables|Default|GetTextChatUiRef)
    (:Is%20Valid
      (bind _result (Default|IsonScreen (.ReturnValue (CallFunction|GetInoUI)) "TextChat"))
      (if _result
        (Default|UpdateConfig (.ReturnValue (CallFunction|GetInoUI)) "TextChat" (Utilities|Struct|MakeST_AUK_Core_InputMode "NewEnumerator4" "NewEnumerator1"))
        (Default|StartMessaging (Variables|Default|GetTextChatUiRef))))))